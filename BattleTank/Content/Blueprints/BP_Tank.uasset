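; BP_Tank is the player-controllable tank, handling camera aim, firing and tracked movement.
; BeginPlay hands the turret, barrel and both tracks to InitialiseComponents.
; Aim axes yaw the horizontal gimbal and pitch the camera arm, scaled by per-axis sensitivity, and the Fire action calls Fire.
; Driving supports two schemes: forward and turn intents routed through TankMovementComponent, or direct throttle on each track.
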(event EventBeginPlay
  (Class|Tank|InitialiseComponents (Variables|Default|GetTurret) (Variables|Default|GetBarrel) (Variables|Default|GetLeft%20Track) (Variables|Default|GetRight%20Track)))

(event Input|ActionEvents|InputActionFire
  (params (Key :type Key%20Structure))
  ;[1 1 1] Aiming
  (:Pressed
    (Class|Tank|Fire)))

(event Input|AxisEvents|InputAxisAimElevation
  (params (AxisValue :type Float%20%28single-precision%29))
  ;[1 1 1] Aiming
  (Transformation|AddRelativeRotation (Variables|Default|GetCamera%20Arm) (Math|Rotator|MakeRotator 0.0 (* (Variables|CameraControls|GetY%20Sensitivity) AxisValue) 0.0) false false))

(event Input|AxisEvents|InputAxisAimHorizon
  (params (AxisValue :type Float%20%28single-precision%29))
  ;[1 1 1] Aiming
  (Transformation|AddRelativeRotation (Variables|Default|GetHorizontal%20Gimbal) (Math|Rotator|MakeRotator 0.0 0.0 (* (Variables|CameraControls|GetX%20Sensitivity) AxisValue)) false false))

(event Input|AxisEvents|InputAxisLeftTrackThrottle
  (params (AxisValue :type Float%20%28single-precision%29))
  ;[1 1 1] Movement
  (Class|TankTrack|SetThrottle (Variables|Default|GetLeft%20Track) AxisValue))

(event Input|AxisEvents|InputAxisRightTrackThrottle
  (params (AxisValue :type Float%20%28single-precision%29))
  ;[1 1 1] Movement
  (Class|TankTrack|SetThrottle (Variables|Default|GetRight%20Track) AxisValue))

(event Input|AxisEvents|InputAxisMoveForward
  (params (AxisValue :type Float%20%28single-precision%29))
  ;[1 1 1] Movement
  (Class|TankMovementComponent|IntendMoveForward (Variables|Default|GetTankMovementComponent) AxisValue))

(event Input|AxisEvents|InputAxisTurnRight
  (params (AxisValue :type Float%20%28single-precision%29))
  ;[1 1 1] Movement
  (Class|TankMovementComponent|IntendTurnRight (Variables|Default|GetTankMovementComponent) AxisValue))

(fn ConstructionScript)